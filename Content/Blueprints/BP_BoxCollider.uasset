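; BP_BoxCollider is an actor that pairs a Box component with an entity component carrying a MassStep box collision trait.
; Its construction script calls ResizeTestBox, which sets the trait's Extents to the box extent multiplied by actor scale, syncing the collider to the box shape.
; The event graph has no active logic.
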(event `self.ReceiveBeginPlay`)

(fn `Resize Test Box`
  (`/Engine/EditorBlueprintResources/StandardMacros.IsValid` (`self.Box`)
    (:`Is Valid`
      (bind _asms_box_collider (cast `MassStepBoxCollisionTrait` (`MassStepEntityComponent.GetTrait` (`self.EntityComponent`) "/Script/MassStepGameplay.MassStepBoxCollisionTrait")))
      (set `MassStepBoxCollisionTrait.Extents` (* (`BoxComponent.BoxExtent` (`self.Box`)) (`self.GetActorScale3D`)) _asms_box_collider))))

(fn `UserConstructionScript`
  (`self.Resize Test Box`))